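; Tavion character Blueprint: a lightsaber-wielding combatant assigned to team 2.
; The construction script initializes the lightsaber and team, then BeginPlay sets force jump to level 2, single-saber arming, the lightsaber style and a reset direction key.
; Hits on the left and right saber colliders against other actors spawn a burst particle at the impact point, oriented along the surface normal.
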(event OnComponentHit(Collider_SaberLeft)
  (params (HitComponent :type Primitive%20Component%20Object%20Reference) (OtherActor :type Actor%20Object%20Reference) (OtherComp :type Primitive%20Component%20Object%20Reference) (NormalImpulse :type Vector :default "0, 0, 0") (Hit :type Hit%20Result%20Structure%20%28by%20ref%29))
  (if (!= OtherActor self)
    (Effects|SpawnEmitteratLocation "/Game/StarterContent/Particles/P_SiingleBurst.P_SiingleBurst" (.location Hit) (Math|Conversions|RotationFromXVector (.normal Hit)))))

(event OnComponentHit(Collider_SaberRight)
  (params (HitComponent :type Primitive%20Component%20Object%20Reference) (OtherActor :type Actor%20Object%20Reference) (OtherComp :type Primitive%20Component%20Object%20Reference) (NormalImpulse :type Vector :default "0, 0, 0") (Hit :type Hit%20Result%20Structure%20%28by%20ref%29))
  (if (!= OtherActor self)
    (Effects|SpawnEmitteratLocation "/Game/StarterContent/Particles/P_SiingleBurst.P_SiingleBurst" (.location Hit) (Math|Conversions|RotationFromXVector (.normal Hit)))))

(event EventBeginPlay
  (Class|JediCharacter|SetForceJump "I_Level2")
  (Class|JediCharacter|SetSaberArmingState "SaberSingle")
  (Variables|Default|SetLightsaberStyle 0)
  (Variables|Default|SetfDirectionKey 0.0))

(event EventActorBeginOverlap
  (params (OtherActor :type Actor%20Object%20Reference)))

(event EventTick
  (params (DeltaSeconds :type Float%20%28single-precision%29)))

(fn ConstructionScript
  (Class|JediCharacter|InitLightsaber)
  (Variables|Default|SetCharacterTeam "T_Team2"))