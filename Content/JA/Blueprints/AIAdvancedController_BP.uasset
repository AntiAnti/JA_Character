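; AI controller for Jedi characters that picks an enemy and starts their behavior tree.
; On BeginPlay it loads Humanoid_BB, reads the controlled character's team, and stores the first JediCharacter on another team as ActiveEnemy.
; It then runs Jedi_BT; the target is chosen only once, without distance or sight checks.
; An unconnected jump-loop and flying-mode test remains in the graph and never runs.
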(event EventBeginPlay
  (Class|AIController|UseBlackboard "/Game/JA/Blueprints/Humanoid_BB.Humanoid_BB")
  ;[1 1 1] Find Enemy
  (bind _asjedi_character (Utilities|Casting|CastToJediCharacter (Pawn|GetControlledPawn)))
  (bind _returnvalue (Class|AcademyCharacter|GetCharacterTeam _asjedi_character))
  (Variables|Default|SetMyTeam _returnvalue)
  (bind _outactors (Actor|GetAllActorsOfClass "/Script/JA_Character.JediCharacter"))
  (bind _array_element (Utilities|Array|ForEachLoopwithBreak _outactors :!label _label)
    (:LoopBody
      (bind _returnvalue_2 (Class|AcademyCharacter|GetCharacterTeam _array_element))
      (if (!= _returnvalue_2 (Variables|Default|GetMyTeam))
        (AI|Components|Blackboard|SetValueasObject (AI|GetBlackboard self) (Variables|Default|GetActiveEnemy) _array_element)
        (goto _label Break)))
    (:Completed
      (AI|RunBehaviorTree "/Game/JA/Blueprints/Jedi_BT.Jedi_BT"))))

(event EventTick
  (params (DeltaSeconds :type Float%20%28single-precision%29)))

(fn ConstructionScript)