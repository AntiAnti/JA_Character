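; EQ_EnemyCharacterContext is an Environment Query context that supplies the querier's enemy characters as a set of actors.
; It gathers every AcademyCharacter in the world and keeps those the querier's IsEnemy check flags as hostile.
; If the querier is not an AcademyCharacter, it returns all AcademyCharacters unfiltered.
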(fn ProvideActorsSet
  (params (QuerierActor :type Actor%20Object%20Reference))
  (bind _asacademy_character (Utilities|Casting|CastToAcademyCharacter QuerierActor)
    (:then
      (bind _outactors (Actor|GetAllActorsOfClass "/Script/JA_Character.AcademyCharacter"))
      (for _array_element _outactors
        (bind _returnvalue (Class|AcademyCharacter|IsEnemy _asacademy_character _array_element))
        (if _returnvalue
          (Utilities|Array|Add (LocalVariables|GetResult) _array_element)))
      (return (LocalVariables|GetResult)))
    (:CastFailed
      (bind _outactors_2 (Actor|GetAllActorsOfClass "/Script/JA_Character.AcademyCharacter"))
      (return _outactors_2))))