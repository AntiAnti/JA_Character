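; Behavior tree task that writes an AI pawn's next target location to a vector blackboard key.
; Despite its name, a FlipFlop alternates the target between two hard-coded world points on successive executions, then the task finishes successfully.
; An unconnected branch that would pick a random navigable point around the pawn remains in the graph but never runs.
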(event EventReceiveExecuteAI
  (params (OwnerController :type AI%20Controller%20Object%20Reference) (ControlledPawn :type Pawn%20Object%20Reference))
  (Utilities|FlowControl|FlipFlop
    (:A
      (AI|BehaviorTree|SetBlackboardValueasVector (Variables|Default|GetKey_VTarget) (Math|Vector|MakeVector -3e+02 8.26e+03 2e+02)))
    (:B
      (AI|BehaviorTree|SetBlackboardValueasVector (Variables|Default|GetKey_VTarget) (Math|Vector|MakeVector -2.7e+02 1.3e+03 2e+02))))
  (AI|BehaviorTree|FinishExecute true))